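; BP_Player is the player pawn for a cursor-aimed shooter, handling movement, shooting, health and pausing.
; Input axes move it along world X and Z, while Tick rotates it toward the cursor trace hit using X and Z.
; Left and right mouse buttons spawn red and blue marks at ArrowShot.
; Damage reaching zero health triggers GameOver on BP_GameState, and pausing works through BP_HUD's pause widget.
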(event `Pick Health`
  (`/Engine/EditorBlueprintResources/StandardMacros.IncrementInt` (`self.Health`)))

(event `Damage`
  (bind _health (`self.Health`))
  ;[1 1 1] Player health value
  (bind _result (`/Engine/EditorBlueprintResources/StandardMacros.DecrementInt` _health)
    (:`  `
      (`KismetSystemLibrary.PrintString` (`KismetStringLibrary.Conv_IntToString` _health))
      (if (<= _result 0)
        (`/Game/Gameplay/BP_GameState.Game Over` (cast `/Game/Gameplay/BP_GameState` (`GameplayStatics.GetGameState`) :!pure true))))))

(event `self.ReceiveTick`
  (params (DeltaSeconds :type "Float (single-precision)"))
  ;[1 1 1] Event Tick
  (if (> (`self.CustomTimeDilation`) 0.0)
    (`self.Aim`)))

(event `InputAxis|MoveRight`
  (params (AxisValue :type "Float (single-precision)"))
  ;[1 1 1] Movement
  (if (> AxisValue 0.0)
    (set `self.bIsMovingRight` true)
    (elif (< AxisValue 0.0)
      (set `self.bIsMovingRight` false)))
  (`self.AddMovementInput` (-1.0 0.0 0.0) AxisValue))

(event `InputAxis|MoveForward`
  (params (AxisValue :type "Float (single-precision)"))
  ;[1 1 1] Movement
  (if (> AxisValue 0.0)
    (set `self.bIsMovingForward` true)
    (elif (< AxisValue 0.0)
      (set `self.bIsMovingForward` false)))
  (`self.AddMovementInput` (0.0 0.0 1.0) AxisValue))

(event `Aim`
  ;[1 1 1] Aim
  (`self.K2_SetActorRotation` (`KismetMathLibrary.FindLookAtRotation` (`KismetMathLibrary.MakeVector` (.x (`self.K2_GetActorLocation`)) 0.0 (.z (`self.K2_GetActorLocation`))) (`KismetMathLibrary.MakeVector` (.x (`.Location` (`GameplayStatics.BreakHitResult` (`PlayerController.GetHitResultUnderCursorByChannel` (`GameplayStatics.GetPlayerController` 0) "TraceTypeQuery2" false)))) 0.0 (.z (`.Location` (`GameplayStatics.BreakHitResult` (`PlayerController.GetHitResultUnderCursorByChannel` (`GameplayStatics.GetPlayerController` 0) "TraceTypeQuery2" false))))))))

(event `InputAction|Pause`
  (params (Key :type "Key Structure"))
  (:`Pressed`
    (`self.PauseGame`)))

(event `Key|LeftMouseButton`
  (params (Key :type "Key Structure"))
  (bind (_returnvalue_location _returnvalue_rotation) (`KismetMathLibrary.BreakTransform` (`SceneComponent.K2_GetComponentToWorld` (`self.ArrowShot`))))
  ;[1 1 1] Shoot Bullets
  (:`Pressed`
    (`|SpawnActorFromClass` "/Game/Weapons/Player/Blueprints/BP_RedMark.BP_RedMark_C" (`KismetMathLibrary.MakeTransform` _returnvalue_location _returnvalue_rotation) "Undefined" "OverrideRootScale" self self)))

(event `Key|RightMouseButton`
  (params (Key :type "Key Structure"))
  (bind (_returnvalue_location _returnvalue_rotation) (`KismetMathLibrary.BreakTransform` (`SceneComponent.K2_GetComponentToWorld` (`self.ArrowShot`))))
  ;[1 1 1] Shoot Bullets
  (:`Pressed`
    (`|SpawnActorFromClass` "/Game/Weapons/Player/Blueprints/BP_BlueMark.BP_BlueMark_C" (`KismetMathLibrary.MakeTransform` _returnvalue_location _returnvalue_rotation) "Undefined" "OverrideRootScale" self self)))

(fn `PauseGame`
  (`GameplayStatics.SetGamePaused` true)
  (`/Game/UI/BP_HUD.Create Pause` (cast `/Game/UI/BP_HUD` (`PlayerController.GetHUD` (`GameplayStatics.GetPlayerController` 0)) :!pure true)))

(fn `UnpauseGame`
  (`GameplayStatics.SetGamePaused` false)
  (`Widget.RemoveFromParent` (`/Game/UI/BP_HUD.WidgetPause Reference` (cast `/Game/UI/BP_HUD` (`PlayerController.GetHUD` (`GameplayStatics.GetPlayerController` 0)) :!pure true)))
  (`WidgetBlueprintLibrary.SetInputMode_GameAndUIEx` (`GameplayStatics.GetPlayerController` 0) null "DoNotLock" false)
  (set `PlayerController.CurrentMouseCursor` "Crosshairs" (cast `/Game/Characters/Player/BP_PlayerController` (`GameplayStatics.GetPlayerController` 0) :!pure true)))

(fn `UserConstructionScript`)