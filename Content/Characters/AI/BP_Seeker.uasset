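; BP_Seeker is an AI character that chases the player pawn and fires at it.
; While PauseTick0 is false, each tick turns it toward player 0, adds movement input in that direction and calls Shoot.
; Shoot relies on Delay ignoring retriggers to space shots about 1.5 seconds apart, spawning a scaled-down BP_SeekerShot and a blaster sound at ArrowShot.
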(event `self.Event Tick Parent`
  ;[1 1 1] Event Tick
  (if (not (`self.Pause Tick_0`))
    (`self.Rotate`)
    (`self.Move`)
    (`self.Shoot`)))

(event `Rotate`
  (bind (_returnvalue_roll _returnvalue_pitch _returnvalue_yaw) (`KismetMathLibrary.BreakRotator` (`KismetMathLibrary.FindLookAtRotation` (`self.K2_GetActorLocation`) (`self.K2_GetActorLocation` (`GameplayStatics.GetPlayerPawn` 0)))))
  ;[1 1 1] Rotate
  (`self.K2_SetActorRotation` (`KismetMathLibrary.MakeRotator` _returnvalue_roll _returnvalue_pitch _returnvalue_yaw)))

(event `Move`
  ;[1 1 1] Move
  (`self.AddMovementInput` (- (`self.K2_GetActorLocation` (`GameplayStatics.GetPlayerPawn` 0)) (`self.K2_GetActorLocation`))))

(event `Shoot`
  (bind (_returnvalue_location _returnvalue_rotation) (`KismetMathLibrary.BreakTransform` (`SceneComponent.K2_GetComponentToWorld` (`self.ArrowShot`))))
  ;[1 1 1] Shoot
  (`KismetSystemLibrary.Delay` 1.5)
  (`|SpawnActorFromClass` "/Game/Weapons/Seeker/Blueprints/BP_SeekerShot.BP_SeekerShot_C" (`KismetMathLibrary.MakeTransform` _returnvalue_location _returnvalue_rotation (0.4 0.4 0.4)) "Undefined" "OverrideRootScale" null null)
  (`GameplayStatics.SpawnSoundAtLocation` "/Game/Sound/SFX/Cue_blaster.Cue_blaster" _returnvalue_location (struct) 0.5 1.0 0.0 null null))

(fn `UserConstructionScript`)