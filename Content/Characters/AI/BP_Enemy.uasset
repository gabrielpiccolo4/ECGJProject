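; Base 2D-sprite enemy that can be marked red or blue so that linked pairs crash into each other.
; Marking swaps the flipbook; once GameMode holds both marks, red simulates physics and a repeating timeline impulses it toward blue.
; Their collision spawns scraps and destroys both, with EndPlay notifying GameState.
; Hidden enemies wait at zero time dilation until SpawnEnemy, which also gates the tick event for children.
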(event `self.ReceiveBeginPlay`
  (if (`self.BeginHidden`)
    (set `self.CustomTimeDilation` 0.0)
    (`self.SetActorHiddenInGame` true)))

(event `self.ReceiveTick`
  (params (DeltaSeconds :type "Float (single-precision)"))
  (if (> (`self.CustomTimeDilation`) 0.0)
    (`self.Event Tick Parent`)))

(event `Event Tick Parent`)

(event `Spawn Enemy`
  (`self.SetActorHiddenInGame` false)
  (`KismetSystemLibrary.Delay` 0.7)
  (set `self.CustomTimeDilation` 1.0))

(event `self.ReceiveEndPlay`
  (params (EndPlayReason :type "EEndPlayReason Enum" :default "Destroyed"))
  (`/Game/Gameplay/BP_GameState.Enemy Destroyed` (cast `/Game/Gameplay/BP_GameState` (`GameplayStatics.GetGameState`) :!pure true))
  (`GameplayStatics.SpawnSoundAtLocation` "/Game/Sound/SFX/Cue_impacts.Cue_impacts" (`self.K2_GetActorLocation`) (struct) 0.5 1.0 0.0 null null))

(event `Mark`
  (params (REd :type Boolean))
  (bind _sprite (`self.Sprite`))
  ;[1 1 1] Mark
  (if REd
    (`KismetSystemLibrary.PrintString` "RedMARKED")
    (`PaperFlipbookComponent.SetFlipbook` _sprite "/Game/Characters/Sprites/SeekerRed_Flipbook.SeekerRed_Flipbook")
    (else
      (`KismetSystemLibrary.PrintString` "BlueMARKED")
      (set `self.Blue` true)
      (`PaperFlipbookComponent.SetFlipbook` _sprite "/Game/Characters/Sprites/SeekerBlue_Flipbook.SeekerBlue_Flipbook")
      (`ActorComponent.Deactivate` (`self.CharacterMovement`))))
  (`self.Link Event`))

(event `SpawnScraps`
  (bind _trace_end_0_0 (`self.Trace End_0_0`))
  ;[1 1 1] Spawn Scraps
  (`|SpawnActorFromClass` "/Game/Weapons/Scraps/Blueprints/BP_Scraps.BP_Scraps_C" (`KismetMathLibrary.MakeTransform` _trace_end_0_0 (`KismetMathLibrary.FindLookAtRotation` (`self.Trace Start_0`) _trace_end_0_0)) "AdjustIfPossibleButAlwaysSpawn" "OverrideRootScale" (`self.GetOwner`) (`self.GetInstigator`)))

(event `LinkMovement`
  ;[1 1 1] Link Movement
  (bind _asbp_game_mode (cast `/Game/Gameplay/BP_GameMode` (`GameplayStatics.GetGameMode`)))
  (bind (_direction _velocity) (`Timeline|Timeline_0` :!via `PlayFromStart` :!label _label)
    (:`Update`
      (bind _red_marked (`/Game/Gameplay/BP_GameMode.Red Marked` _asbp_game_mode))
      (`PrimitiveComponent.AddImpulse` (`Character.CapsuleComponent` _red_marked) (* (- (`self.Trace End`) (`self.K2_GetActorLocation` _red_marked)) _velocity) "None" false))
    (:`Finished`
      (`KismetSystemLibrary.Delay` 0.2)
      (goto _label :!via `PlayFromStart`))))

(event `Unmark`
  (params (Red :type Boolean))
  ;[1 1 1] Unmask
  (if Red
    (set `self.Pause Tick` false)
    (else
      (`ActorComponent.Activate` (`self.CharacterMovement`) false)))
  (`KismetSystemLibrary.PrintString` "UNMARKED")
  (`PrimitiveComponent.SetMaterial` (`self.Sprite`) 0 "/Game/Characters/AI/Materials/MI_SeekerBase.MI_SeekerBase"))

(event `Link Event`
  ;[1 1 1] Link Event
  (bind _asbp_game_mode (cast `/Game/Gameplay/BP_GameMode` (`GameplayStatics.GetGameMode`)))
  (bind _red_marked (`/Game/Gameplay/BP_GameMode.Red Marked` _asbp_game_mode))
  (`/Engine/EditorBlueprintResources/StandardMacros.IsValid` _red_marked
    (:`Is Valid`
      (bind _blue_marked (`/Game/Gameplay/BP_GameMode.Blue Marked` _asbp_game_mode))
      (`/Engine/EditorBlueprintResources/StandardMacros.IsValid` _blue_marked
        (:`Is Valid`
          (set `self.Trace Start` (`self.K2_GetActorLocation` _red_marked))
          (set `self.Trace End_0` (`self.K2_GetActorLocation` _blue_marked))
          (bind _red_marked_2 (`/Game/Gameplay/BP_GameMode.Red Marked` _asbp_game_mode))
          (set `/Game/Characters/AI/BP_Enemy.Pause Tick` true _red_marked_2)
          (`PrimitiveComponent.SetSimulatePhysics` (`Character.CapsuleComponent` _red_marked_2) true)
          (`self.LinkMovement`))))))

(event `self.CapsuleComponent.OnComponentHit`
  (params (HitComponent :type "PrimitiveComponent Object Reference") (OtherActor :type "Actor Object Reference") (OtherComp :type "PrimitiveComponent Object Reference") (NormalImpulse :type "Vector Structure") (Hit :type "HitResult Structure (by ref)"))
  ;[1 1 1] Destroy Actors
  (bind _asbp_game_mode (cast `/Game/Gameplay/BP_GameMode` (`GameplayStatics.GetGameMode`)))
  (bind _asbp_enemy (cast `/Game/Characters/AI/BP_Enemy` OtherActor))
  (bind _blue_marked (`/Game/Gameplay/BP_GameMode.Blue Marked` _asbp_game_mode))
  (bind _red_marked (`/Game/Gameplay/BP_GameMode.Red Marked` _asbp_game_mode))
  (if (and (== _asbp_enemy _blue_marked) (== _red_marked self))
    (set `self.Trace Start_0_0` (`self.K2_GetActorLocation` _red_marked))
    (set `self.Trace End_0_0_0` (`self.K2_GetActorLocation` _blue_marked))
    (`self.SpawnScraps`)
    (`GameplayStatics.SpawnSoundAtLocation` "/Game/Sound/SFX/Cue_impacts.Cue_impacts" (`self.K2_GetActorLocation`) (struct) 0.5 1.0 0.0 null null)
    (`self.K2_DestroyActor` _red_marked)
    (`self.K2_DestroyActor` _blue_marked)))

(fn `UserConstructionScript`)