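; BP_Scraps is a weapon actor, apparently a projectile, that bursts into scatter projectiles on impact.
; When its Collision component registers a hit, it spawns one BP_ScatterProjectiles per entry in AnglesToSpawn, then destroys itself.
; Each child spawns at the actor's location, with a rotation derived from the actor's own and that entry, and inherits its owner and instigator.
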(event `self.Collision.OnComponentHit`
  (params (HitComponent :type "PrimitiveComponent Object Reference") (OtherActor :type "Actor Object Reference") (OtherComp :type "PrimitiveComponent Object Reference") (NormalImpulse :type "Vector Structure") (Hit :type "HitResult Structure (by ref)"))
  (`self.Spawn Projetiles`)
  (`self.K2_DestroyActor`))

(event `Spawn Projetiles`
  (for _array_element (`self.AnglesToSpawn`)
    (`|SpawnActorFromClass` "/Game/Weapons/Scraps/Blueprints/BP_ScatterProjectiles.BP_ScatterProjectiles_C" (`KismetMathLibrary.MakeTransform` (`self.K2_GetActorLocation`) (* (`self.K2_GetActorRotation`) _array_element)) "Undefined" "OverrideRootScale" (`self.GetOwner`) (`self.GetInstigator`))))

(fn `UserConstructionScript`)