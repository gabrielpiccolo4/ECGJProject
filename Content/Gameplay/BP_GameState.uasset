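; Game state Blueprint that handles room-clearing progression and game over.
; On EnemyDestroyed, it gathers the RoomIDs of surviving enemies, then checks a fixed set of four room indices.
; For each empty room, trigger rooms one ID below it open their doors, and each match flags all scatter-projectile actors as finished.
; GameOver pauses the game and has the HUD create the game-over screen.
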(event `Enemy Destroyed`
  (`KismetArrayLibrary.Array_Clear` (`self.CurrentExistingRoomID`))
  (bind _outactors (`GameplayStatics.GetAllActorsOfClass` "/Game/Characters/AI/BP_Enemy.BP_Enemy_C"))
  (for _array_element _outactors
    (if (not (`self.IsActorBeingDestroyed` _array_element))
      (bind _returnvalue (`KismetArrayLibrary.Array_AddUnique` (`self.CurrentExistingRoomID`) (`/Game/Characters/AI/BP_Enemy.RoomID` _array_element)))
      (if (== _returnvalue 2)
        (`KismetSystemLibrary.PrintString` (`KismetStringLibrary.Conv_IntToString` _returnvalue) true true (struct :`R` 0.195311 :`G` 1.0 :`A` 1.0) 5.0))))
  (`|ExecutionSequence`
    (:`then_0`
      (set `self.CurrentRoomBeingTested` 0))
    (:`then_1`
      (set `self.CurrentRoomBeingTested` 1))
    (:`then_2`
      (set `self.CurrentRoomBeingTested` 2))
    (:`then_3`
      (set `self.CurrentRoomBeingTested` 3)))
  (if (== (`KismetArrayLibrary.Array_Find` (`self.CurrentExistingRoomID`) (`self.CurrentRoomBeingTested`)) -1)
    (bind _outactors_2 (`GameplayStatics.GetAllActorsOfClass` "/Game/Gameplay/Blueprints/BP_TriggerRoom.BP_TriggerRoom_C"))
    (for _array_element_2 _outactors_2
      (if (== (+ (`/Game/Gameplay/Blueprints/BP_TriggerRoom.RoomID` _array_element_2) 1) (`self.CurrentRoomBeingTested`))
        (`/Game/Gameplay/Blueprints/BP_TriggerRoom.OpenDoor` _array_element_2)
        (bind _outactors_3 (`GameplayStatics.GetAllActorsOfClass` "/Game/Weapons/Scraps/Blueprints/BP_ScatterProjectiles.BP_ScatterProjectiles_C"))
        (for _array_element_3 _outactors_3
          (set `/Game/Weapons/Scraps/Blueprints/BP_ScatterProjectiles.Finish` true _array_element_3))))))

(event `Game Over`
  (`GameplayStatics.SetGamePaused` true)
  (`/Game/UI/BP_HUD.Create GameOver` (cast `/Game/UI/BP_HUD` (`PlayerController.GetHUD` (`GameplayStatics.GetPlayerController` 0)) :!pure true)))

(fn `UserConstructionScript`)