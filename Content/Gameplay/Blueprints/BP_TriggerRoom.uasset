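; BP_TriggerRoom is a door trigger that transitions the camera and player into the room matching its RoomID.
; On player overlap, a timeline slides the camera in X and Z to that room's BP_CamTargetPoint while the player's time dilation is zeroed.
; A one-shot timeline moves the input-disabled player to an arrow.
; A second trigger spawns the room's enemies, and the door's open state sets its material and collision at BeginPlay.
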(event `self.ReceiveActorBeginOverlap`
  (params (OtherActor :type "Actor Object Reference"))
  ;[1 1 1] Move the camera to the next level
  (cast `/Game/Characters/Player/BP_Player` OtherActor)
  (bind _outactors (`GameplayStatics.GetAllActorsOfClass` "/Game/Gameplay/Blueprints/BP_CamTargetPoint.BP_CamTargetPoint_C"))
  (for _array_element _outactors :!label _label
    (set `self.TargetPoint Reference` _array_element)
    (if (== (`/Game/Gameplay/Blueprints/BP_CamTargetPoint.RoomID` (`self.TargetPoint Reference`)) (`self.RoomID`))
      (`self.BreakLoop`)
      (bind _outactors_2 (`GameplayStatics.GetAllActorsOfClass` "/Game/Gameplay/Blueprints/BP_CameraActor.BP_CameraActor_C"))
      (set `self.CameraActor Reference` (`|GetArrayItem` _outactors_2))
      (if (!= (`/Game/Gameplay/Blueprints/BP_CameraActor.CurrentRoomID` (`self.CameraActor Reference`)) (`self.RoomID`))
        (set `self.CurrentCameraLocation` (`self.K2_GetActorLocation` (`self.CameraActor Reference`)))
        (set `/Game/Gameplay/Blueprints/BP_CameraActor.CurrentRoomID` (`self.RoomID`) (`self.CameraActor Reference`))
        (`self.Freeze Actors` 0.0)
        (`self.Move`)
        (bind (_direction _newtrack_2) (`Timeline|TimelineCameraMove` :!via `PlayFromStart`)
          (:`Update`
            (`self.K2_SetActorLocation` (`self.CameraActor Reference`) (`KismetMathLibrary.VLerp` (`self.CurrentCameraLocation`) (`self.Target Camera Location`) _newtrack_2) true false))
          (:`Finished`
            (`KismetSystemLibrary.Delay` 1.0)
            (`self.Freeze Actors` 1.0)))
        (else
          (`KismetSystemLibrary.PrintString` "NEXT CAMERA POINT LOCATION NOT FOUND" true true (struct :`R` 1.0 :`G` 0.035028 :`A` 1.0) 10.0))))))

(event `BreakLoop`
  ;[1 1 1] Move the camera to the next level
  (goto _label :!via `Break`))

(event `self.ReceiveBeginPlay`
  ;[1 1 1] Begin Play
  (set `self.DoorStartLocation` (`SceneComponent.RelativeLocation` (`self.Cube`)))
  (if (`self.bIsDoorOpen`)
    (`self.OpenDoor`)
    (else
      (`self.Close Door`))))

(event `Freeze Actors`
  (params (CustomTimeDilation :type "Float (double-precision)"))
  ;[1 1 1] Set Time Dilation
  (set `Actor.CustomTimeDilation` CustomTimeDilation (cast `/Game/Characters/Player/BP_Player` (`GameplayStatics.GetPlayerCharacter` 0) :!pure true)))

(event `Close Door`
  ;[1 1 1] Open / Close Doors
  (`PrimitiveComponent.SetMaterial` (`self.Cube`) 0 "/Game/Weapons/Player/Materials/MI_RedBullet.MI_RedBullet")
  (`PrimitiveComponent.SetCollisionResponseToAllChannels` (`self.Box`) "ECR_Block"))

(event `self.ReceiveActorEndOverlap`
  (params (OtherActor :type "Actor Object Reference"))
  ;[1 1 1] Close Door
)

(event `OpenDoor`
  ;[1 1 1] Open / Close Doors
  (`PrimitiveComponent.SetMaterial` (`self.Cube`) 0 "/Game/Weapons/Player/Materials/MI_BlueBullet.MI_BlueBullet")
  (`PrimitiveComponent.SetCollisionResponseToAllChannels` (`self.Box`) "ECR_Overlap"))

(event `Move`
  (bind _returnvalue (`self.K2_GetActorLocation` (`GameplayStatics.GetPlayerCharacter` 0)))
  (bind _asbp_player_controller (cast `/Game/Characters/Player/BP_PlayerController` (`GameplayStatics.GetPlayerController` 0) :!pure true))
  (bind _asbp_player_controller_2 (cast `/Game/Characters/Player/BP_PlayerController` (`GameplayStatics.GetPlayerController` 0) :!pure true))
  ;[1 1 1] Player movement transaction from one side of the door to the other
  (`/Engine/EditorBlueprintResources/StandardMacros.DoOnce` false
    (:`Completed`
      (`self.DisableInput` _asbp_player_controller_2 _asbp_player_controller_2)
      (set `self.PlayerCurrentLocation` _returnvalue)
      (`Controller.SetControlRotation` (`GameplayStatics.GetPlayerController` 0) (`KismetMathLibrary.FindLookAtRotation` _returnvalue (`SceneComponent.K2_GetComponentLocation` (`self.Arrow1`))))
      (bind (_direction _newtrack_2) (`Timeline|Timeline_0` :!via `PlayFromStart`)
        (:`Update`
          (`self.K2_SetActorLocation` (`GameplayStatics.GetPlayerCharacter` 0) (`KismetMathLibrary.VLerp` (`self.PlayerCurrentLocation`) (`SceneComponent.K2_GetComponentLocation` (`self.Arrow1`)) _newtrack_2) true false))
        (:`Finished`
          (`self.EnableInput` _asbp_player_controller _asbp_player_controller))))))

(event `self.SpawnEnemies.OnComponentBeginOverlap`
  (params (OverlappedComponent :type "PrimitiveComponent Object Reference") (OtherActor :type "Actor Object Reference") (OtherComp :type "PrimitiveComponent Object Reference") (OtherBodyIndex :type Integer) (bFromSweep :type Boolean) (SweepResult :type "HitResult Structure (by ref)"))
  ;[1 1 1] Spawn enemies inside the room
  (cast `/Game/Characters/Player/BP_Player` OtherActor)
  (`KismetSystemLibrary.Delay` 0.3)
  (bind _outactors (`GameplayStatics.GetAllActorsOfClass` "/Game/Characters/AI/BP_Enemy.BP_Enemy_C"))
  (for _array_element _outactors
    (if (== (`/Game/Characters/AI/BP_Enemy.RoomID` _array_element) (`self.RoomID`))
      (`/Game/Characters/AI/BP_Enemy.Spawn Enemy` _array_element))))

(fn `Target Camera Location`
  (returns (ReturnValue :type "Vector Structure"))
  (return (`KismetMathLibrary.MakeVector` (.x (`self.K2_GetActorLocation` (`self.TargetPoint Reference`))) (.y (`self.CurrentCameraLocation`)) (.z (`self.K2_GetActorLocation` (`self.TargetPoint Reference`))))))

(fn `UserConstructionScript`)