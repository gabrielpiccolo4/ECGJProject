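; Game mode that tracks one red-marked and one blue-marked enemy at a time.
; RedMark and BlueMark accept a BP_Enemy that is not being destroyed and reject one already holding the other color.
; A valid target replaces the previous one of that color: UnMark clears the old enemy's mark and HasMarked flag, then the new enemy is stored and marked.
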(event `RedMark`
  (params (EnemyToMark :type "Actor Object Reference"))
  (set `self.New Target` null)
  (bind _asbp_enemy (cast `/Game/Characters/AI/BP_Enemy` EnemyToMark))
  (if (not (`self.IsActorBeingDestroyed` _asbp_enemy))
    (bind _output_get (set `self.New Target` _asbp_enemy))
    (if (not (== _output_get (`self.Blue Marked`)))
      (`self.UnMark` (`self.Red Marked`) true)
      (bind _output_get_2 (set `self.Red Marked` (`self.New Target`)))
      (`/Game/Characters/AI/BP_Enemy.Mark` _output_get_2 true))))

(event `BlueMark`
  (params (EnemyToMark :type "Actor Object Reference"))
  (set `self.New Target` null)
  (bind _asbp_enemy (cast `/Game/Characters/AI/BP_Enemy` EnemyToMark))
  (if (not (`self.IsActorBeingDestroyed` _asbp_enemy))
    (bind _output_get (set `self.New Target` _asbp_enemy))
    (if (not (== _output_get (`self.Red Marked`)))
      (`self.UnMark` (`self.Blue Marked`))
      (bind _output_get_2 (set `self.Blue Marked` (`self.New Target`)))
      (`/Game/Characters/AI/BP_Enemy.Mark` _output_get_2 false))))

(event `UnMark`
  (params (Target :type "Actor Object Reference") (IsRed :type Boolean))
  (bind _asbp_enemy (cast `/Game/Characters/AI/BP_Enemy` Target))
  (`/Game/Characters/AI/BP_Enemy.Unmark` _asbp_enemy IsRed)
  (set `/Game/Characters/AI/BP_Enemy.HasMarked` false _asbp_enemy))

(fn `UserConstructionScript`)